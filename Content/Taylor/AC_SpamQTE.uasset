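; Actor component running a quick-time event on WBP_SpamQTE, pairing a key-mash challenge with a timing challenge, each on a randomly chosen key.
; Mashing fills a bar to a random target; a retriggerable delay after key release fails it, and either result calls CallCompleted and destroys the component.
; The timing key checks a ping-ponging slider's X position, then shows a random good or bad splash with sound from data tables.
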(event `self.ReceiveBeginPlay`
  (bind _spamwidgetref (`self.SpamWidgetRef`))
  (bind _spamwidgetref_2 (`self.SpamWidgetRef`))
  (bind _slideanim (`/Game/Taylor/Widgets/WBP_SpamQTE.SlideAnim` _spamwidgetref))
  (bind _slideanim_2 (`/Game/Taylor/Widgets/WBP_SpamQTE.SlideAnim` _spamwidgetref_2))
  ;[0.2658 0.4682 1 0.5] Main line of code for the Spam QTE
  (`self.SplashRef`
    (:`then`)
    (:`else`
      (`self.SpamWidgetRef`
        (:`then`)
        (:`else`
          (`|ExecutionSequence`
            (:`then_0`
              (bind _returnvalue (`|CreateWidget` "/Game/Taylor/Widgets/WBP_SpamQTE.WBP_SpamQTE_C"))
              (bind _output_get (set `self.SpamWidgetRef` _returnvalue))
              (`UserWidget.AddToViewport` _output_get 0)
              (set `self.NeededAmount` (`KismetMathLibrary.RandomFloatInRange` 10.0 15.0))
              (set `self.KeyPressed` (select `int` (`KismetMathLibrary.RandomInteger` 3) :`0` "E" :`1` "V" :`2` "F" :!type "Key Structure"))
              (`TextBlock.SetText` (`/Game/Taylor/Widgets/WBP_SpamQTE.TXT_KEY` (`self.SpamWidgetRef`)) (`|FormatText` "\"{Key}\"" (`KismetInputLibrary.Key_GetDisplayName` (`self.KeyPressed`))))
              (`self.UpdateSpamBar`)
              (`KismetSystemLibrary.Delay` 5.0)
              (`/Engine/EditorBlueprintResources/StandardMacros.IsValid` self
                (:`Is Valid`
                  (if (<= (`self.PressedAmount`) 0.0)
                    (if (or (== (`self.Key`) "E") (== (`self.Key`) "V") (== (`self.Key`) "F"))
                      (`self.OnFailed`))))))
            (:`then_1`
              (set `self.keyforp` (select `int` (`KismetMathLibrary.RandomInteger` 3) :`0` "T" :`1` "H" :`2` "X" :!type "Key Structure"))
              (`|ExecutionSequence`
                (:`then_0`
                  (`TextBlock.SetText` (`/Game/Taylor/Widgets/WBP_SpamQTE.TXT_PKEY` (`self.SpamWidgetRef`)) (`|FormatText` "\"{Key}\"" (`KismetInputLibrary.Key_GetDisplayName` (`self.keyforp`))))
                  (`UserWidget.PlayAnimation` _spamwidgetref_2 _slideanim_2 0.0 1 "Forward" 1.0 false :!label _label)
                  (`KismetSystemLibrary.Delay` (+ (`WidgetAnimation.GetEndTime` _slideanim_2) 0.1))
                  (`UserWidget.PlayAnimation` _spamwidgetref _slideanim 0.0 1 "Reverse" 1.0 false)
                  (`KismetSystemLibrary.Delay` (+ (`WidgetAnimation.GetEndTime` _slideanim) 0.1))
                  (`self.LoopAnim`))))
            (:`then_2`
              (`self.SplashRef`
                (:`then`)
                (:`else`
                  (if (not true)
                    (`KismetSystemLibrary.Delay` 5.0)
                    (if (not (`self.SuccessP`))
                      (`self.Fail P QTE` false))))))))))))

(event `LoopAnim`
  ;[0.2658 0.4682 1 0.5] Main line of code for the Spam QTE
  (goto _label))

(event `PressedKey`
  ;[0.2658 0.4682 1 0.5] PressedKey
  (bind _result (`/Engine/EditorBlueprintResources/StandardMacros.IncrementFloat` (`self.PressedAmount`))
    (:`  `
      (set `self.PressedAmount` (`KismetMathLibrary.FClamp` _result 0.0 (`self.NeededAmount`)))
      (`self.UpdateSpamBar`)
      (if (== (`self.PressedAmount`) (`self.NeededAmount`))
        (`self.Completed` true)
        (`self.Destroy`)))))

(event `OnFailed`
  ;[0.2658 0.4682 1 0.5] When the QTE fails
  (set `self.PressedAmount` 0.0)
  (`self.UpdateSpamBar`)
  (`self.Completed` false)
  (`self.Destroy`))

(event `ReleasedKey`
  ;[0.2658 0.4682 1 0.5] Key not pressed
  (`KismetSystemLibrary.RetriggerableDelay` 0.8)
  (`self.OnFailed`))

(event `Destroy`
  ;[0.2658 0.4682 1 0.5] Remove AC and end interaction
  (bind _spamwidgetref (`self.SpamWidgetRef`)
    (:`then`
      (`Widget.RemoveFromParent` _spamwidgetref)
      (`self.K2_DestroyComponent`))
    (:`else`)))

(event `Key|AnyKey`
  (params (Key :type "Key Structure"))
  (bind _splashref (`self.SplashRef`))
  (bind _splashref_2 (`self.SplashRef`))
  (bind _x (`KismetMathLibrary.BreakVector2D` (`.Translation` (break `WidgetTransform` (`Widget.RenderTransform` (`/Game/Taylor/Widgets/WBP_SpamQTE.IMG_SLIDER` (`self.SpamWidgetRef`)))))))
  ;[0.2658 0.4682 1 0.5] Manual key functions
  (:`Pressed`
    (bind _output_get (set `self.Key` Key))
    (`|ExecutionSequence`
      (:`then_0`
        (if (== _output_get (`self.KeyPressed`))
          (`self.PressedKey`)))
      (:`then_1`
        ;[0.2819 0.01496 0.75 0.5] PQTE OUTPUT
        (if (== _output_get (`self.keyforp`))
          (`/Engine/EditorBlueprintResources/StandardMacros.DoOnce` false :!label _label_2
            (:`Completed`
              (if (and (> _x 225.0) (< _x 255.0))
                (`KismetSystemLibrary.PrintString` "Success")
                (set `self.SuccessP` true)
                (`Widget.RemoveFromParent` (`self.SpamWidgetRef`))
                ;[0.01678 0.8854 0.001505 0.5] P QTE WIN
                (bind _returnvalue (`|CreateWidget` "/Game/Taylor/Widgets/WBP_Splash.WBP_Splash_C"))
                (bind _output_get_2 (set `self.SplashRef` _returnvalue))
                (bind _outrownames (`DataTableFunctionLibrary.GetDataTableRowNames` "/Game/Taylor/Data/DT_GoodSplash.DT_GoodSplash"))
                (bind _returnvalue_2 (`|GetDataTableRow` "/Game/Taylor/Data/DT_GoodSplash.DT_GoodSplash" (`KismetArrayLibrary.Array_Random` _outrownames))
                  (:`then`
                    (`Image.SetBrushFromTexture` (`/Game/Taylor/Widgets/WBP_Splash.IMG_Splash` _output_get_2) (break `/Game/Taylor/Data/F_SplashArt` _returnvalue_2) false)
                    (`GameplayStatics.PlaySound2D` (`.Sound_6_E116F04B434360B34F2D378E8B5200C3` (break `/Game/Taylor/Data/F_SplashArt` _returnvalue_2)) 1.0 1.0 0.0 null null)
                    (`UserWidget.AddToViewport` _splashref 0)
                    (`KismetSystemLibrary.Delay` 3.0)
                    (`Widget.RemoveFromParent` _splashref)))
                (else
                  (`KismetSystemLibrary.PrintString` "Failure" :!label _label_3)
                  (`Widget.RemoveFromParent` (`self.SpamWidgetRef`))
                  ;[1 0 0 0.5] P QTE LOSE
                  (bind _returnvalue_3 (`|CreateWidget` "/Game/Taylor/Widgets/WBP_Splash.WBP_Splash_C"))
                  (bind _output_get_3 (set `self.SplashRef` _returnvalue_3))
                  (bind _outrownames_2 (`DataTableFunctionLibrary.GetDataTableRowNames` "/Game/Taylor/Data/DT_BadSplash.DT_BadSplash"))
                  (bind _returnvalue_4 (`|GetDataTableRow` "/Game/Taylor/Data/DT_BadSplash.DT_BadSplash" (`KismetArrayLibrary.Array_Random` _outrownames_2))
                    (:`then`
                      (`Image.SetBrushFromTexture` (`/Game/Taylor/Widgets/WBP_Splash.IMG_Splash` _output_get_3) (break `/Game/Taylor/Data/F_SplashArt` _returnvalue_4) false)
                      (`GameplayStatics.PlaySound2D` (`.Sound_6_E116F04B434360B34F2D378E8B5200C3` (break `/Game/Taylor/Data/F_SplashArt` _returnvalue_4)) 1.0 1.0 0.0 null null)
                      (`UserWidget.AddToViewport` _splashref_2 0)
                      (`KismetSystemLibrary.Delay` 3.0)
                      (`Widget.RemoveFromParent` _splashref_2)))))))
          (else
            (goto _label_2 :!via `Reset`))))))
  (:`Released`
    (if (== _output_get (`self.KeyPressed`))
      (`self.ReleasedKey`))))

(event `Fail P QTE`
  (params (`Completed?` :type Boolean))
  ;[0.2819 0.01496 0.75 0.5] PQTE OUTPUT
  (if (not `Completed?`)
    (goto _label_3)))

(fn `UpdateSpamBar`
  ;[0 0.05679 1] Update progress bar
  (`ProgressBar.SetPercent` (`/Game/Taylor/Widgets/WBP_SpamQTE.PB_PROGRESSBAR` (`self.SpamWidgetRef`)) (/ (`self.PressedAmount`) (`self.NeededAmount`))))