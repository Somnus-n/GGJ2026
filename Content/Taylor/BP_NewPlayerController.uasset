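; Player controller that adds a mouse-driven arm mode to the third-person character.
; Holding left mouse enables ArmMode, also setting the character's flag on press, though release clears only the controller's copy.
; While active, mouse axis input scaled by sensitivity accumulates into a clamped MousePosition.
; On BeginPlay it caches the pawn and hands itself to the mesh's ABP_Lean animation Blueprint.
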(event `Key|LeftMouseButton`
  (params (Key :type "Key Structure"))
  (:`Pressed`
    (set `self.ArmMode` true)
    (set `/Game/ThirdPerson/Blueprints/BP_ThirdPersonCharacter.ArmMode` true (`self.ThirdPersonCharacter`)))
  (:`Released`
    (set `self.ArmMode` false)))

(event `InputVectorAxis|Mouse2D`
  (params (AxisValue :type "Vector Structure"))
  (bind (_returnvalue_x _returnvalue_y) (`KismetMathLibrary.BreakVector` (+ (* (`self.MouseSensitivity`) AxisValue) (`self.MousePosition`))))
  (if (`self.ArmMode`)
    (set `self.MousePosition` (`KismetMathLibrary.MakeVector` (`KismetMathLibrary.FClamp` _returnvalue_x -50.0 50.0) (`KismetMathLibrary.FClamp` _returnvalue_y -30.0 20.0)))))

(event `self.ReceiveBeginPlay`
  (bind _asbp_third_person_character (cast `/Game/ThirdPerson/Blueprints/BP_ThirdPersonCharacter` (`self.K2_GetPawn`)))
  (bind _output_get (set `self.ThirdPersonCharacter` _asbp_third_person_character))
  (bind _asabp_lean (cast `/Game/Taylor/Animations/ABP_Lean` (`SkeletalMeshComponent.GetAnimInstance` (`Character.Mesh` _output_get))))
  (set `/Game/Taylor/Animations/ABP_Lean.PlayerController` self _asabp_lean))

(fn `UserConstructionScript`)